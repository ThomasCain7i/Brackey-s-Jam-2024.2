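; Base enemy for a tower defense game that walks a waypoint path and damages the MainTower at the end.
; BeginPlay sets walk speed, then chains AIMoveTo through all TargetPoints from last array index to zero.
; At index zero it reduces tower health, calls WaveManager's enemy count check and destroys itself.
; A self-recalling 0.1s event tracks distance to the current waypoint, while a damage event handles health and death.
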(event `self.ReceiveBeginPlay`
  (`self.DistanceChecker`)
  (`KismetSystemLibrary.Delay` 0.1)
  (set `CharacterMovementComponent.MaxWalkSpeed` (`self.Speed`) (`self.CharacterMovement`))
  (bind _outactors (`GameplayStatics.GetAllActorsOfClass` "/Script/Engine.TargetPoint"))
  (bind _output_get (set `self.WaypointIndex` (- (`KismetArrayLibrary.Array_Length` _outactors) 1)))
  (bind _output (`|GetArrayItem` _outactors _output_get))
  (set `self.CurrentWaypoint` _output :!label _label)
  (`|AIMoveTo` self (0.0 0.0 0.0) _output 100.0
    (:`OnSuccess`
      (if (== (`self.WaypointIndex`) 0)
        (bind _returnvalue (`GameplayStatics.GetActorOfClass` "/Game/WreckzFolder/Blueprints/MainTower/MainTower.MainTower_C"))
        (set `/Game/WreckzFolder/Blueprints/MainTower/MainTower.MainHealth` (- (`/Game/WreckzFolder/Blueprints/MainTower/MainTower.MainHealth` _returnvalue) (`self.Damage`)) _returnvalue)
        (bind _returnvalue_2 (`GameplayStatics.GetActorOfClass` "/Game/WreckzFolder/Blueprints/WaveSpawner/WaveManager.WaveManager_C"))
        (`/Game/WreckzFolder/Blueprints/WaveSpawner/WaveManager.CheckHowManyEnmies` _returnvalue_2)
        (`self.K2_DestroyActor`)
        (else
          (set `self.WaypointIndex` (- (`self.WaypointIndex`) 1))
          (goto _label))))))

(event `DistanceChecker`
  (set `self.DistanceToNextWaypoint` (`KismetMathLibrary.Vector_Distance` (`self.K2_GetActorLocation` (`self.CurrentWaypoint`)) (`self.K2_GetActorLocation` self)))
  (`KismetSystemLibrary.Delay` 0.1)
  (`self.DistanceChecker`))

(event `TakeDamage_Event`
  (params (Damage :type "Float (double-precision)"))
  (bind _returnvalue (- (`self.CurrentHealth`) Damage))
  (set `self.CurrentHealth` _returnvalue)
  (if (<= _returnvalue 0.0)
    (`self.K2_DestroyActor`)))

(fn `UserConstructionScript`)