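; ShieldEnemy is an enemy Blueprint that grants shielded status to nearby enemies within its sphere collision.
; On overlap, it casts actors tagged "Enemy" to BaseEnemy and sets their Shielded flag if not already set.
; When they leave the sphere, a short delay runs before the flag is cleared, with debug prints marking both changes.
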(event `self.Sphere.OnComponentBeginOverlap`
  (params (OverlappedComponent :type "PrimitiveComponent Object Reference") (OtherActor :type "Actor Object Reference") (OtherComp :type "PrimitiveComponent Object Reference") (OtherBodyIndex :type Integer) (bFromSweep :type Boolean) (SweepResult :type "HitResult Structure (by ref)"))
  (if (`self.ActorHasTag` OtherActor "Enemy")
    (bind _asbase_enemy (cast `/Game/WreckzFolder/Blueprints/Enemies/BaseEnemy` OtherActor))
    (if (not (`/Game/WreckzFolder/Blueprints/Enemies/BaseEnemy.Shielded?` _asbase_enemy))
      (set `/Game/WreckzFolder/Blueprints/Enemies/BaseEnemy.Shielded?` true _asbase_enemy)
      (`KismetSystemLibrary.PrintString` "Shielded"))))

(event `self.Sphere.OnComponentEndOverlap`
  (params (OverlappedComponent :type "PrimitiveComponent Object Reference") (OtherActor :type "Actor Object Reference") (OtherComp :type "PrimitiveComponent Object Reference") (OtherBodyIndex :type Integer))
  (if (`self.ActorHasTag` OtherActor "Enemy")
    (bind _asbase_enemy (cast `/Game/WreckzFolder/Blueprints/Enemies/BaseEnemy` OtherActor))
    (`KismetSystemLibrary.Delay` 0.25)
    (set `/Game/WreckzFolder/Blueprints/Enemies/BaseEnemy.Shielded?` false _asbase_enemy)
    (`KismetSystemLibrary.PrintString` "UnShielded")))

(fn `UserConstructionScript`
  (`parent.UserConstructionScript`))