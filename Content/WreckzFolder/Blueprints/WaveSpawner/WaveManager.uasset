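; WaveManager is an actor intended to spawn enemy waves, still unfinished.
; On BeginPlay it counts actors tagged "Enemy" and calls SpawnWave when none are found; the count is not repeated afterwards.
; SpawnWave only reaches an enum switch with no actions attached.
; A node that spawns a BaseEnemy AI at the manager's location is present but disconnected, so no enemies spawn.
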(event `self.ReceiveBeginPlay`
  (`self.CheckHowManyEnmies`))

(event `CheckHowManyEnmies`
  (bind _outactors (`GameplayStatics.GetAllActorsWithTag` "Enemy"))
  (bind _output_get (set `self.Number Of Enemies` (`KismetArrayLibrary.Array_Length` _outactors)))
  (if (== _output_get 0)
    (`self.Spawn Wave`)))

(event `Spawn Wave`
  (switch `|SwitchEnum` 0))

(fn `UserConstructionScript`)